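; Modular interactive door that cycles through closed, part-open and open states, swinging away from or toward closed on each interaction.
; Interaction picks the swing side from the dot product of the player's forward vector and the door's open-location arrow.
; While interaction is active, Tick interpolates door yaw toward the target for the current state.
; A timer then stops the motion and advances the state enum.
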(event `self.ReceiveBeginPlay`
  (bind _asbp_first_person_character (cast `/Game/FirstPerson/Blueprints/BP_FirstPersonCharacter` (`GameplayStatics.GetPlayerCharacter` 0)))
  (set `self.Char REF` _asbp_first_person_character))

(event `self.ReceiveTick`
  (params (DeltaSeconds :type "Float (single-precision)"))
  (if (`self.BIsInteractWithDoor?`)
    (`self.Handle door`)))

(event `Handlerotation of door`
  (params (`set rotation` :type "Float (double-precision)"))
  ;[0.15 0.01063 0.05628 0.5] handle rotation
  (`SceneComponent.K2_SetRelativeRotation` (`self.door`) (`KismetMathLibrary.MakeRotator` 0.0 0.0 (`KismetMathLibrary.FInterpTo` (.yaw (`SceneComponent.RelativeRotation` (`self.door`))) `set rotation` (`GameplayStatics.GetWorldDeltaSeconds`) (`self.Interp Speed`))) false false)
  (`KismetSystemLibrary.PrintString` "Hello"))

(event `Handle door`
  ; Handle door (rotating door acc current state)
  (switch `/Game/BP_trigger/E_Doorstates` (`self.EDoorStates`)
    (:`NewEnumerator0`
      (`self.Handlerotation of door` (* 15.0 (`self.Door OPen Side`))))
    (:`NewEnumerator1`
      (`self.Handlerotation of door` (* (`self.Door Open Angle`) (`self.Door OPen Side`))))
    (:`NewEnumerator2`
      (`self.Handlerotation of door` 0.0))))

(event `IsInteractingwithDoor`
  (params (Player :type "/Game/FirstPerson/Blueprints/BP_FirstPersonCharacter Object Reference"))
  ; doorinteraction Math
  (if (> (`KismetMathLibrary.Dot_VectorVector` (`self.GetActorForwardVector` Player) (`SceneComponent.GetForwardVector` (`self.doorOpenlocation`))) 0.0)
    (set `self.Door OPen Side` 1.0)
    (else
      (set `self.Door OPen Side` -1.0)))
  (set `self.BIsInteractWithDoor?` true)
  (`KismetSystemLibrary.K2_SetTimerDelegate` (delegate `CustomEvent`) (`self.door soundTime`)))

(event `CustomEvent`
  ; doorinteraction Math
  (set `self.BIsInteractWithDoor?` false)
  (switch `/Game/BP_trigger/E_Doorstates` (`self.EDoorStates`)
    (:`NewEnumerator0`
      (set `self.EDoorStates` "NewEnumerator1"))
    (:`NewEnumerator1`
      (set `self.EDoorStates` "NewEnumerator2"))
    (:`NewEnumerator2`
      (set `self.EDoorStates` "NewEnumerator0"))))

(fn `UserConstructionScript`)