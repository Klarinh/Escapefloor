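; BP_Fenster is a window that swings open with a banging noise when anything overlaps its Hghg component.
; The overlap plays a timeline that yaws one mesh, and each update also calls Play on a second timeline that yaws the other mesh the opposite way.
; A DoOnce on the second timeline's update plays the attenuated sound at the actor's location only once, with no reset or closing logic.
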(event `self.hghg.OnComponentBeginOverlap`
  (params (OverlappedComponent :type "PrimitiveComponent Object Reference") (OtherActor :type "Actor Object Reference") (OtherComp :type "PrimitiveComponent Object Reference") (OtherBodyIndex :type Integer) (bFromSweep :type Boolean) (SweepResult :type "HitResult Structure (by ref)"))
  (bind (_direction _windows_float) (`Timeline|Timeline`)
    (:`Update`
      (`SceneComponent.K2_SetRelativeRotation` (`self.StaticMesh2`) (`KismetMathLibrary.MakeRotator` 0.0 0.0 (`KismetMathLibrary.Lerp` 0.0 -160.0 _windows_float)) false false)
      (bind (_direction_2 _windows_float_2) (`Timeline|openwindows`)
        (:`Update`
          (`SceneComponent.K2_SetRelativeRotation` (`self.StaticMesh44`) (`KismetMathLibrary.MakeRotator` 0.0 0.0 (`KismetMathLibrary.Lerp` 0.0 140.0 _windows_float_2)) false false)
          (`/Engine/EditorBlueprintResources/StandardMacros.DoOnce` false
            (:`Completed`
              (`GameplayStatics.PlaySoundAtLocation` "/Game/Sound/672388__melloja__banging-noise.672388__melloja__banging-noise" (`self.K2_GetActorLocation`) (struct) 0.8 1.0 0.0 "/Game/Sound/local_attenuation1.local_attenuation1" null null null))))))))

(fn `UserConstructionScript`)