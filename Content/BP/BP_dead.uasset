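; BP_dead is an interactable rope prop, apparently part of a death scene, that reacts when the player or another object comes near.
; Overlapping the Fj component plays a hangman's-rope sound at the actor and runs a timeline that tilts the Rope component up to 15 degrees in roll.
; Interacting creates a UI_Dialogbox showing the player's inspect line, "What's that?".
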(event `self.fj.OnComponentBeginOverlap`
  (params (OverlappedComponent :type "PrimitiveComponent Object Reference") (OtherActor :type "Actor Object Reference") (OtherComp :type "PrimitiveComponent Object Reference") (OtherBodyIndex :type Integer) (bFromSweep :type Boolean) (SweepResult :type "HitResult Structure (by ref)"))
  (`GameplayStatics.PlaySoundAtLocation` "/Game/Sound/254735__jergonda__hang-mans-rope.254735__jergonda__hang-mans-rope" (`self.K2_GetActorLocation`) (struct) 0.6 1.0 0.0 "/Game/Sound/local_attenuation.local_attenuation" null null null)
  (bind (_direction _newtrack_0) (`Timeline|Timelinerope`)
    (:`Update`
      (`SceneComponent.K2_SetRelativeRotation` (`self.rope`) (`KismetMathLibrary.MakeRotator` (`KismetMathLibrary.Lerp` 0.0 -15.0 _newtrack_0)) false false)
      (`/Engine/EditorBlueprintResources/StandardMacros.DoOnce` false))))

(event `/Game/FirstPerson/Blueprints/InteractInterface.On Interact`
  (params (Interactor :type "/Game/FirstPerson/Blueprints/BP_FirstPersonCharacter Object Reference"))
  (bind _returnvalue (`|CreateWidget` "/Game/UI/UI_Dialogbox.UI_Dialogbox_C" (`GameplayStatics.GetPlayerController` 0) "You" "What's that?"))
  (`UserWidget.AddToViewport` _returnvalue 0)
  (message `/Game/FirstPerson/Blueprints/InteractInterface.Inspect` _returnvalue null null "" ""))

(fn `UserConstructionScript`)