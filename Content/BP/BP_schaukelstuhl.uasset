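; Rocking chair prop that reacts to overlaps with its trigger box using sound and motion.
; Begin overlap plays an attenuated creak sound and starts a Timeline that lerps the mesh's pitch to tilt it.
; End overlap plays an old music box sound at the actor's location.
; DoOnce nodes sit at the chain ends with nothing after them, so both sounds can retrigger.
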(event `self.Box1.OnComponentBeginOverlap`
  (params (OverlappedComponent :type "PrimitiveComponent Object Reference") (OtherActor :type "Actor Object Reference") (OtherComp :type "PrimitiveComponent Object Reference") (OtherBodyIndex :type Integer) (bFromSweep :type Boolean) (SweepResult :type "HitResult Structure (by ref)"))
  (`GameplayStatics.PlaySoundAtLocation` "/Game/Sound/80475__stevelalonde__rockingchair3.80475__stevelalonde__rockingchair3" (`self.K2_GetActorLocation`) (struct) 1.0 1.0 0.0 "/Game/Sound/local_attenuation.local_attenuation" null null null)
  (bind (_direction _newtrack_0) (`Timeline|Timeline`)
    (:`Update`
      (`SceneComponent.K2_SetRelativeRotation` (`self.StaticMesh`) (`KismetMathLibrary.MakeRotator` 0.0 (`KismetMathLibrary.Lerp` 0.0 -25.0 _newtrack_0)) false false)
      (`/Engine/EditorBlueprintResources/StandardMacros.DoOnce` false))))

(event `self.Box1.OnComponentEndOverlap`
  (params (OverlappedComponent :type "PrimitiveComponent Object Reference") (OtherActor :type "Actor Object Reference") (OtherComp :type "PrimitiveComponent Object Reference") (OtherBodyIndex :type Integer))
  (`GameplayStatics.PlaySoundAtLocation` "/Game/Sound/366161__pastabra__old-music-box.366161__pastabra__old-music-box" (`self.K2_GetActorLocation`) (struct) 1.0 1.0 0.0 "/Game/Sound/local_attenuation.local_attenuation" null null null)
  (`/Engine/EditorBlueprintResources/StandardMacros.DoOnce` false))

(fn `UserConstructionScript`)