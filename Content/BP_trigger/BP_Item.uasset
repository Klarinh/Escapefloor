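; BP_Item is an item actor that shows proximity interaction indicators as the player approaches.
; Two collision spheres, sized from radius variables in the construction script, toggle inner and outer indicator visibility.
; The player entering the inner sphere swaps the outer indicator for the inner one, and leaving swaps back.
; Any overlapping actor reveals the outer indicator, but only the player leaving the outer sphere hides it.
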(event `self.innerspherecollision.OnComponentBeginOverlap`
  (params (OverlappedComponent :type "PrimitiveComponent Object Reference") (OtherActor :type "Actor Object Reference") (OtherComp :type "PrimitiveComponent Object Reference") (OtherBodyIndex :type Integer) (bFromSweep :type Boolean) (SweepResult :type "HitResult Structure (by ref)"))
  (if (== OtherActor (`GameplayStatics.GetPlayerCharacter` 0))
    (`SceneComponent.SetVisibility` (`self.innerinteract`) true false)
    (`SceneComponent.SetVisibility` (`self.outerinteract`) false false)))

(event `self.innerspherecollision.OnComponentEndOverlap`
  (params (OverlappedComponent :type "PrimitiveComponent Object Reference") (OtherActor :type "Actor Object Reference") (OtherComp :type "PrimitiveComponent Object Reference") (OtherBodyIndex :type Integer))
  (if (== OtherActor (`GameplayStatics.GetPlayerCharacter` 0))
    (`SceneComponent.SetVisibility` (`self.innerinteract`) false false)
    (`SceneComponent.SetVisibility` (`self.outerinteract`) true false)))

(event `self.outerspherecollison.OnComponentBeginOverlap`
  (params (OverlappedComponent :type "PrimitiveComponent Object Reference") (OtherActor :type "Actor Object Reference") (OtherComp :type "PrimitiveComponent Object Reference") (OtherBodyIndex :type Integer) (bFromSweep :type Boolean) (SweepResult :type "HitResult Structure (by ref)"))
  (if true
    (`SceneComponent.SetVisibility` (`self.outerinteract`) true false)))

(event `self.outerspherecollison.OnComponentEndOverlap`
  (params (OverlappedComponent :type "PrimitiveComponent Object Reference") (OtherActor :type "Actor Object Reference") (OtherComp :type "PrimitiveComponent Object Reference") (OtherBodyIndex :type Integer))
  (if (== (`GameplayStatics.GetPlayerCharacter` 0) OtherActor)
    (`SceneComponent.SetVisibility` (`self.outerinteract`) false false)))

(fn `UserConstructionScript`
  (`SphereComponent.SetSphereRadius` (`self.innerspherecollision`) (`self.Innersphere Radius`) true)
  (`SphereComponent.SetSphereRadius` (`self.outerspherecollison`) (`self.Outersphere Radius_0`) true))