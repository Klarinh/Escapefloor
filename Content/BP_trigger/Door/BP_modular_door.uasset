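; Modular door actor that the first-person player swings through closed, part-open and open states, each with its own sound.
; Tick detects interaction on this door, then interpolates yaw until a timer advances the state.
; A dot product of player and door forward vectors picks the swing side.
; Optional auto-close shuts an open door with one interpolation step after the player leaves the trigger box facing along world Y.
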(event `self.ReceiveBeginPlay`
  (bind _asbp_first_person_character (cast `/Game/FirstPerson/Blueprints/BP_FirstPersonCharacter` (`GameplayStatics.GetPlayerCharacter` 0)))
  (set `self.Char REF` _asbp_first_person_character))

(event `self.ReceiveTick`
  (params (DeltaSeconds :type "Float (single-precision)"))
  (bind _char_ref (`self.Char REF`))
  (if (and (`/Game/FirstPerson/Blueprints/BP_FirstPersonCharacter.Is Interacting?` _char_ref) (== (`/Game/FirstPerson/Blueprints/BP_FirstPersonCharacter.Hit Actor` _char_ref) self))
    (if (`self.BIsInteractWithDoor?`)
      (`self.Handle door`)
      (else
        (`self.IsInteractingwithDoor` (`self.Char REF`))))))

(event `Handlerotation of door`
  (params (`set rotation` :type "Float (double-precision)"))
  ;[0.15 0.01063 0.05628 0.5] handle rotation
  (`SceneComponent.K2_SetRelativeRotation` (`self.door`) (`KismetMathLibrary.MakeRotator` 0.0 0.0 (`KismetMathLibrary.FInterpTo` (.yaw (`SceneComponent.RelativeRotation` (`self.door`))) `set rotation` (`GameplayStatics.GetWorldDeltaSeconds`) (`self.Interp Speed`))) false false))

(event `Handle door`
  ; Handle door (rotating door acc current state)
  (switch `/Game/BP_trigger/Door/E_Doorstates` (`self.EDoorStates`)
    (:`NewEnumerator0`
      (`self.Handlerotation of door` (* 15.0 (`self.Door OPen Side`)))
      (set `self.doorOpen?` true))
    (:`NewEnumerator1`
      (`self.Handlerotation of door` (* (`self.Door Open Angle`) (`self.Door OPen Side`)))
      (set `self.doorOpen?` true))
    (:`NewEnumerator2`
      (if (== (`self.Door OPen Side`) 1.0)
        (`self.Handlerotation of door` -5.0)
        (set `self.doorOpen?` false)
        (else
          (`self.Handlerotation of door` 5.0)
          (set `self.doorOpen?` false))))))

(event `Door States Sounds`
  (bind _returnvalue (`self.K2_GetActorLocation`))
  ; sounds
  (switch `/Game/BP_trigger/Door/E_Doorstates` (`self.EDoorStates`)
    (:`NewEnumerator0`
      (`GameplayStatics.PlaySoundAtLocation` "/Game/Sound/door/104533__skyumori__door_open_02.104533__skyumori__door_open_02" _returnvalue (struct) 1.0 1.0 0.0 null null null null))
    (:`NewEnumerator1`
      (`GameplayStatics.PlaySoundAtLocation` "/Game/Sound/door/270219__jagadamba__door-creaking-01.270219__jagadamba__door-creaking-01" _returnvalue (struct) 1.0 1.0 0.0 null null null null))
    (:`NewEnumerator2`
      (`GameplayStatics.PlaySoundAtLocation` "/Game/Sound/door/752064__qubodup__creepy-door-closing.752064__qubodup__creepy-door-closing" _returnvalue (struct) 1.0 1.0 0.0 null null null null))))

(event `IsInteractingwithDoor`
  (params (Player :type "/Game/FirstPerson/Blueprints/BP_FirstPersonCharacter Object Reference"))
  ; doorinteraction Math
  (if (`self.Auto closed activated`)
    (set `self.EDoorStates` "NewEnumerator0")
    (set `self.Auto closed activated` false))
  (`self.Door States Sounds`)
  (if (> (`KismetMathLibrary.Dot_VectorVector` (`self.GetActorForwardVector` Player) (`SceneComponent.GetForwardVector` (`self.doorOpenlocation`))) 0.0)
    (set `self.Door OPen Side` 1.0)
    (else
      (set `self.Door OPen Side` -1.0)))
  (set `self.BIsInteractWithDoor?` true)
  (`KismetSystemLibrary.K2_SetTimerDelegate` (delegate `CustomEvent`) (`self.door soundTime`)))

(event `CustomEvent`
  ; doorinteraction Math
  (set `self.BIsInteractWithDoor?` false)
  (switch `/Game/BP_trigger/Door/E_Doorstates` (`self.EDoorStates`)
    (:`NewEnumerator0`
      (set `self.EDoorStates` "NewEnumerator1"))
    (:`NewEnumerator1`
      (set `self.EDoorStates` "NewEnumerator2"))
    (:`NewEnumerator2`
      (set `self.EDoorStates` "NewEnumerator0"))))

(event `self.Box.OnComponentEndOverlap`
  (params (OverlappedComponent :type "PrimitiveComponent Object Reference") (OtherActor :type "Actor Object Reference") (OtherComp :type "PrimitiveComponent Object Reference") (OtherBodyIndex :type Integer))
  (bind _returnvalue (`GameplayStatics.GetPlayerCharacter` 0))
  (bind (_returnvalue_x _returnvalue_y) (`KismetMathLibrary.BreakVector` (`self.GetActorForwardVector` _returnvalue)))
  ; Closing auto
  (if (and (`self.Autoclose?`) (`self.doorOpen?`))
    (if (and (== OtherActor _returnvalue) (or (>= _returnvalue_y 0.7) (<= _returnvalue_y -0.7)))
      (`KismetSystemLibrary.Delay` 0.5)
      (`self.Autocloseddoor`)
      (set `self.Auto closed activated` true))))

(event `Autocloseddoor`
  ; Closing auto
  ;; Close door Functionality
  (`GameplayStatics.PlaySoundAtLocation` "/Game/Sound/door/752064__qubodup__creepy-door-closing.752064__qubodup__creepy-door-closing" (`self.K2_GetActorLocation`) (struct) 1.0 1.0 0.0 null null null null)
  (`SceneComponent.K2_SetRelativeRotation` (`self.door`) (`KismetMathLibrary.MakeRotator` 0.0 0.0 (`KismetMathLibrary.FInterpTo` (.yaw (`SceneComponent.RelativeRotation` (`self.door`))) 0.0 5.0 (`self.Interp Speed`))) false false))

(fn `UserConstructionScript`)